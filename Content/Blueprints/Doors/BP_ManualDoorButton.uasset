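; BP_ManualDoorButton is an interactable button that toggles its assigned door.
; Each Interact flips a state that sets the lock on a LockingDoor (inverted, so the first press unlocks) or opens and closes a ManualDoor.
; Focus and interaction events are forwarded to a WBP_InteractionCard widget.
; If flagged as ping origin, it writes the widget's world location to the MPC_DoorPhase Epicenter parameter on BeginPlay.
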(event `self.ReceiveBeginPlay`
  (if (`self.AmPingOrigin?`)
    (`KismetMaterialLibrary.SetVectorParameterValue` "/Game/Material/MPC_DoorPhase.MPC_DoorPhase" "Epicenter" (`KismetMathLibrary.Conv_VectorToLinearColor` (`SceneComponent.K2_GetComponentLocation` (`self.Widget`))))))

(event `self.Interact`
  (bind _mydoor (`self.MyDoor`))
  ;[1 1 1] Wish I had taken the extra time to make a base class right about now lol
  ; BUT..! It's just for demonstartion purposes; please forgive me
  (bind _isa (`/Engine/EditorBlueprintResources/StandardMacros.FlipFlop`)
    (:`A`
      _)
    (:`B`
      _))
  (bind _aslocking_door (cast `LockingDoor` _mydoor)
    (:`then`
      (`LockingDoor.LockDoor` _aslocking_door (not _isa)))
    (:`CastFailed`
      (bind _asmanual_door (cast `ManualDoor` _mydoor))
      (`ManualDoor.OpenDoor` _asmanual_door _isa))))

(event `self.SetIsFocus`
  (params (bIsFocus :type Boolean))
  (bind _aswbp_interaction_card (cast `/Game/UI/WBP_InteractionCard` (`WidgetComponent.GetWidget` (`self.Widget`))))
  (`/Game/UI/WBP_InteractionCard.Is Focus` _aswbp_interaction_card bIsFocus))

(event `self.OnInteract`
  (bind _aswbp_interaction_card (cast `/Game/UI/WBP_InteractionCard` (`WidgetComponent.GetWidget` (`self.Widget`))))
  (`/Game/UI/WBP_InteractionCard.OnInteracted` _aswbp_interaction_card))

(fn `UserConstructionScript`)