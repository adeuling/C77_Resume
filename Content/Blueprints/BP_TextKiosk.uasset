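; BP_TextKiosk is an interactable kiosk actor that shows or hides a linked text object.
; OnInteract toggles MyTextObject's hidden state and notifies the WBP_InteractionCard in its widget component.
; SetIsFocus forwards focus state to that same card.
; A client-only billboard routine to turn the widget toward the player camera exists but is unconnected, with a note to move it to C++.
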(event `self.ReceiveTick`
  (params (DeltaSeconds :type "Float (single-precision)")))

(event `self.SetIsFocus`
  (params (bIsFocus :type Boolean))
  (bind _aswbp_interaction_card (cast `/Game/UI/WBP_InteractionCard` (`WidgetComponent.GetWidget` (`self.Widget`))))
  (`/Game/UI/WBP_InteractionCard.Is Focus` _aswbp_interaction_card bIsFocus))

(event `self.OnInteract`
  (bind _mytextobject (`self.MyTextObject`))
  (`self.SetActorHiddenInGame` _mytextobject (not (`Actor.bHidden` _mytextobject)))
  (bind _aswbp_interaction_card (cast `/Game/UI/WBP_InteractionCard` (`WidgetComponent.GetWidget` (`self.Widget`))))
  (`/Game/UI/WBP_InteractionCard.OnInteracted` _aswbp_interaction_card))

(event `self.Interact`)

(fn `UserConstructionScript`)